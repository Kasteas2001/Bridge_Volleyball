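; BP_GameMode runs the volleyball match rules, tracking HP against a loss and Score against a win target.
; RepNotify handlers on HP and Score update the HUD counters and, at zero HP or NeedScore, show the final text and fire game over or win.
; Either outcome calls FinishGame, which notifies pawns as winners or losers by team and destroys the ball, then swaps the play sound for a result sound.
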(event Custom|Event_GameOver
  (CallFunction|FinishGame "NewEnumerator1")
  (Audio|Components|Audio|Stop (Variables|Default|GetCurrentSound))
  (Components|DestroyComponent (Variables|Default|GetCurrentSound))
  (bind _returnvalue (Audio|SpawnSound2D "/Game/Valleyball/Blueprints/Sounds/Sound_Lose.Sound_Lose" 1.0 1.0 0.0 0))
  (Variables|Default|SetCurrentSound _returnvalue))

(event Custom|Event_Win
  (CallFunction|FinishGame "NewEnumerator0")
  (Audio|Components|Audio|Stop (Variables|Default|GetCurrentSound))
  (Components|DestroyComponent (Variables|Default|GetCurrentSound))
  (bind _returnvalue (Audio|SpawnSound2D "/Game/Valleyball/Blueprints/Sounds/Sound_Win.Sound_Win" 1.0 1.0 0.0 0))
  (Variables|Default|SetCurrentSound _returnvalue))

(event EventBeginPlay
  (bind _asbp_hud (Utilities|Casting|CastToBP_HUD (HUD|GetHUD (Game|GetPlayerController 0))))
  (Variables|Default|SetAs%20BP%20HUD _asbp_hud)
  (Utilities|FlowControl|Delay 0.1)
  (Variables|Default|SetHP (Variables|Default|GetMaxHP))
  (bind _returnvalue (Audio|SpawnSound2D "/Game/Valleyball/Blueprints/Sounds/Sound_Play.Sound_Play" 1.0 1.0 0.0 0))
  (Variables|Default|SetCurrentSound _returnvalue))

(event EventTick
  (params (DeltaSeconds :type Float%20%28single-precision%29)))

(fn ConstructionScript)

(fn OnRepHP
  (if (== (Variables|Default|GetHP) 0)
    (CallFunction|EventGameOver)
    (bind _as_bp_hud (Variables|Default|GetAs%20BP%20HUD)
      (:then
        (Rendering|Components|TextRender|SetText (Variables|/Game/Valleyball/Blueprints/UI/WB_HUD.WB_HUD_C|GetFinal_Text (Variables|/Game/Valleyball/Blueprints/Core/BP_HUD.BP_HUD_C|GetWB_HUD _as_bp_hud)) "YOU LOSE")
        (Variables|/Script/UMG.TextBlock|SetColorAndOpacity (Variables|/Game/Valleyball/Blueprints/UI/WB_HUD.WB_HUD_C|GetFinal_Text (Variables|/Game/Valleyball/Blueprints/Core/BP_HUD.BP_HUD_C|GetWB_HUD _as_bp_hud)) (Utilities|Struct|MakeSlateColor "(R=1.000000,G=0.000000,B=0.024906,A=1.000000)" "UseColor_Specified")))
      (:else)))
  (bind _as_bp_hud_2 (Variables|Default|GetAs%20BP%20HUD)
    (:then
      (Rendering|Components|TextRender|SetText (Variables|/Game/Valleyball/Blueprints/UI/WB_HUD.WB_HUD_C|GetMiss_Byte (Variables|/Game/Valleyball/Blueprints/Core/BP_HUD.BP_HUD_C|GetWB_HUD _as_bp_hud_2)) (Utilities|Text|ToText(String) (Variables|Default|GetHP))))
    (:else)))

(fn OnRepScore
  (if (>= (Variables|Default|GetScore) (Variables|Default|GetNeedScore))
    (CallFunction|EventWin)
    (bind _as_bp_hud (Variables|Default|GetAs%20BP%20HUD)
      (:then
        (Rendering|Components|TextRender|SetText (Variables|/Game/Valleyball/Blueprints/UI/WB_HUD.WB_HUD_C|GetFinal_Text (Variables|/Game/Valleyball/Blueprints/Core/BP_HUD.BP_HUD_C|GetWB_HUD _as_bp_hud)) "YOU WIN")
        (Variables|/Script/UMG.TextBlock|SetColorAndOpacity (Variables|/Game/Valleyball/Blueprints/UI/WB_HUD.WB_HUD_C|GetFinal_Text (Variables|/Game/Valleyball/Blueprints/Core/BP_HUD.BP_HUD_C|GetWB_HUD _as_bp_hud)) (Utilities|Struct|MakeSlateColor "(R=0.000000,G=1.000000,B=0.007759,A=1.000000)" "UseColor_Specified")))
      (:else)))
  (bind _as_bp_hud_2 (Variables|Default|GetAs%20BP%20HUD)
    (:then
      (Rendering|Components|TextRender|SetText (Variables|/Game/Valleyball/Blueprints/UI/WB_HUD.WB_HUD_C|GetScore_byte (Variables|/Game/Valleyball/Blueprints/Core/BP_HUD.BP_HUD_C|GetWB_HUD _as_bp_hud_2)) (Utilities|Text|ToText(String) (Variables|Default|GetScore))))
    (:else)))

(fn FinishGame
  (params (Winner :type ENUM_Teams%20Enum :default "NewEnumerator0"))
  (bind _outactors (Actor|GetAllActorsOfClass "/Game/Valleyball/Blueprints/Pawn/BP_BaseValleyBallPawn.BP_BaseValleyBallPawn_C"))
  (for _array_element _outactors
    (if (not (Utilities|Enum|Equal(Enum) (Variables|/Game/Valleyball/Blueprints/Pawn/BP_BaseValleyBallPawn.BP_BaseValleyBallPawn_C|GetTeam _array_element) Winner))
      (Default|EventLooser _array_element)
      (else
        (Default|EventWinner _array_element))))
  (bind _returnvalue (Actor|GetActorOfClass "/Game/Valleyball/Blueprints/Actors/BP_Ball.BP_Ball_C"))
  (Utilities|IsValid _returnvalue
    (:Is%20Valid
      (Actor|DestroyActor _returnvalue))))