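; Base volleyball pawn with separate body, head and hand parts that handles pushing and win or lose reactions.
; Tick yaws it toward BallRef, or spins it slowly without a valid ball.
; A sped-up PushAnim timeline is set to pitch RootHands forward, then reverse back to rest.
; Winner event replays the push in an endless delayed loop, while loser event enables physics on the parts and flings them apart with a force.
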(event Custom|Event_Push
  ;[1 1 1] PushBall
  (Components|Timeline|PlayfromStart (Variables|Default|GetPushAnim)))

(event Custom|Event_Looser
  (Physics|SetSimulatePhysics (Variables|Default|GetBody) true)
  (Class|PrimitiveComponent|AddForceatLocationLocal (Variables|Default|GetLeftHand) "200.000000,200.000000,200.000000" (Transformation|GetActorLocation) "None"))

(event Custom|Event_Winner
  (Components|Timeline|PlayfromStart (Variables|Default|GetPushAnim) :!label _label)
  (Utilities|FlowControl|Delay 1.0)
  (Components|Timeline|PlayfromStart (Variables|Default|GetPushAnim))
  (goto _label))

(event EventBeginPlay
  (Components|Timeline|SetPlayRate (Variables|Default|GetPushAnim) 3.0))

(event Collision|EventActorBeginOverlap
  (params (OtherActor :type Actor%20Object%20Reference)))

(event EventTick
  (params (DeltaSeconds :type Float%20%28single-precision%29))
  (bind _ball_ref (Variables|Default|GetBall_Ref)
    (:then
      (Transformation|SetActorRotation (Math|Rotator|MakeRotator 0.0 0.0 (.Yaw (Math|Rotator|BreakRotator (Math|Rotator|FindLookatRotation (Transformation|GetActorLocation) (Transformation|GetActorLocation _ball_ref)))))))
    (:else
      (Transformation|AddActorLocalRotation "0.000000,2.000000,0.000000" false false))))

(fn ConstructionScript)