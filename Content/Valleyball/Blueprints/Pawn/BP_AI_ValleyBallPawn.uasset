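; AI-controlled volleyball pawn that automatically returns the ball when it comes within reach.
; When a BP_Ball overlaps BallTrigger and the stored BallRef is valid, it fires EventPush, then calls SetNewTarget on BallRef with its Team.
; BeginPlay, Tick and actor overlap are disabled stubs, so the trigger overlap is the only active logic in this graph.
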(event OnComponentBeginOverlap(BallTrigger)
  (params (OverlappedComponent :type Primitive%20Component%20Object%20Reference) (OtherActor :type Actor%20Object%20Reference) (OtherComp :type Primitive%20Component%20Object%20Reference) (OtherBodyIndex :type Integer) (bFromSweep :type Boolean) (SweepResult :type Hit%20Result%20Structure%20%28by%20ref%29))
  (if (== (Utilities|GetClass OtherActor) "/Game/Valleyball/Blueprints/Actors/BP_Ball.BP_Ball_C")
    (bind _ball_ref (Variables|Default|GetBall_Ref)
      (:then
        (CallFunction|EventPush)
        (Default|SetNewTarget _ball_ref (Variables|Default|GetTeam)))
      (:else))))

(event EventBeginPlay
  (|CallParentFunction) ; Этот узел отключен и не будет вызываться.\nПеретащите контакты, чтобы построить функционал.
)

(event Collision|EventActorBeginOverlap
  (params (OtherActor :type Actor%20Object%20Reference))
  (|CallParentFunction OtherActor) ; Этот узел отключен и не будет вызываться.\nПеретащите контакты, чтобы построить функционал.
)

(event EventTick
  (params (DeltaSeconds :type Float%20%28single-precision%29))
  (|CallParentFunction DeltaSeconds) ; Этот узел отключен и не будет вызываться.\nПеретащите контакты, чтобы построить функционал.
)

(fn ConstructionScript
  (|CallParentFunction))