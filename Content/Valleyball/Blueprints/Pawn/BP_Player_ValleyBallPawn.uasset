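; Player-controlled pawn for the ValleyBall game, extending a parent pawn with input, scoring and damage.
; The push input runs the parent push unless animating or stunned; a ball inside BallTrigger gets retargeted by team and adds game-mode score.
; A ball hitting HitCollision is also retargeted, but costs game-mode HP and briefly stuns the pawn.
; After a win or loss, the push input reloads the level.
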(event OnComponentBeginOverlap(HitCollision)
  (params (OverlappedComponent :type Primitive%20Component%20Object%20Reference) (OtherActor :type Actor%20Object%20Reference) (OtherComp :type Primitive%20Component%20Object%20Reference) (OtherBodyIndex :type Integer) (bFromSweep :type Boolean) (SweepResult :type Hit%20Result%20Structure%20%28by%20ref%29))
  (if (== (Utilities|GetClass OtherActor) "/Game/Valleyball/Blueprints/Actors/BP_Ball.BP_Ball_C")
    (Default|SetNewTarget (Variables|Default|GetBall_Ref) (Variables|Default|GetTeam))
    (Audio|PlaySound2D "/Engine/EditorSounds/Notifications/CompileFailed.CompileFailed" 1.0 1.0 0.0 0 0)
    (bind _as_bp_game_mode (Variables|Default|GetAs%20BP%20Game%20Mode)
      (:then
        (Variables|/Game/Valleyball/Blueprints/Core/BP_GameMode.BP_GameMode_C|SetHP _as_bp_game_mode (- (Variables|/Game/Valleyball/Blueprints/Core/BP_GameMode.BP_GameMode_C|GetHP _as_bp_game_mode) 1))
        (Variables|Default|SetStan true)
        (Utilities|FlowControl|Delay 0.2)
        (Variables|Default|SetStan false))
      (:else))))

(event EventBeginPlay
  (|CallParentFunction)
  (bind _asbp_game_mode (Utilities|Casting|CastToBP_GameMode (Game|GetGameMode)))
  (Variables|Default|SetAs%20BP%20Game%20Mode _asbp_game_mode))

(event Collision|EventActorBeginOverlap
  (params (OtherActor :type Actor%20Object%20Reference))
  (|CallParentFunction OtherActor) ; Этот узел отключен и не будет вызываться.\nПеретащите контакты, чтобы построить функционал.
)

(event EventTick
  (params (DeltaSeconds :type Float%20%28single-precision%29))
  (|CallParentFunction DeltaSeconds) ; Этот узел отключен и не будет вызываться.\nПеретащите контакты, чтобы построить функционал.
)

(event EventEventPush
  (bind _as_bp_game_mode (Variables|Default|GetAs%20BP%20Game%20Mode))
  (if (and (not (Audio|Components|Audio|IsPlaying (Variables|Default|GetPushAnim))) (not (Variables|Default|GetStan)))
    (|CallParentFunction)
    (if (Collision|IsOverlappingActor (Variables|Default|GetBallTrigger) (Variables|Default|GetBall_Ref) :!class /Script/Engine.PrimitiveComponent)
      (Default|SetNewTarget (Variables|Default|GetBall_Ref) (Variables|Default|GetTeam))
      (Audio|PlaySound2D "/Engine/VREditor/Sounds/VR_open.VR_open" 1.0 1.0 0.0 0 0)
      (Variables|/Game/Valleyball/Blueprints/Core/BP_GameMode.BP_GameMode_C|SetScore _as_bp_game_mode (+ (Variables|/Game/Valleyball/Blueprints/Core/BP_GameMode.BP_GameMode_C|GetScore _as_bp_game_mode) 1)))))

(event EventEventWinner
  (|CallParentFunction)
  (Variables|Default|SetIsGameFinish true))

(event EventEventLooser
  (|CallParentFunction)
  (Variables|Default|SetIsGameFinish true))

(event Input|ActionEvents|InputActionPushBall
  (params (Key :type Key%20Structure :default "None"))
  (:Pressed
    (if (not (Variables|Default|GetIsGameFinish))
      (CallFunction|EventPush)
      (else
        (Game|OpenLevel(byName) "ValleyBall")))))

(fn ConstructionScript
  (|CallParentFunction))