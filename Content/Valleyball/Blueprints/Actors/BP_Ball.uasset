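; BP_Ball is the volleyball actor that flies toward a randomly chosen pawn's position on the opposing team.
; Each tick it faces the target and moves by local offset without physics, climbing until half the horizontal distance remains, then heading straight in.
; SetNewTarget takes the pushing team and stores the new target and starting distance.
; A bot-selection counter restricts one team's push to player targets once it reaches its limit.
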(event Custom|SetNewTarget
  (params (PushedTeam :type ENUM_Teams%20Enum :default "NewEnumerator0"))
  (bind _returnvalue (CallFunction|ChooseNewTargetAfterPush PushedTeam))
  (Variables|Default|SetTarget _returnvalue)
  (Variables|Default|SetStartDistance2D (Math|Vector|Distance2D(Vector) (Transformation|GetActorLocation) (Variables|Default|GetTarget))))

(event EventBeginPlay
  (CallFunction|SetNewTarget "NewEnumerator1"))

(event Collision|EventActorBeginOverlap
  (params (OtherActor :type Actor%20Object%20Reference)))

(event EventTick
  (params (DeltaSeconds :type Float%20%28single-precision%29))
  (bind _returnvalue (Transformation|GetActorLocation))
  (bind _target (Variables|Default|GetTarget))
  (bind _returnvalue_2 (Math|Rotator|FindLookatRotation _returnvalue _target))
  (bind (_roll _pitch _yaw) (Math|Rotator|BreakRotator _returnvalue_2))
  (Transformation|SetActorRotation (Math|Rotator|MakeRotator _roll _pitch _yaw))
  (Transformation|AddActorLocalOffset (* DeltaSeconds (Variables|Default|GetSpeed) (Math|Vector|SelectVector "4.000000,0.000000,0.000000" "3.000000,0.000000,3.000000" (<= (Math|Vector|Distance2D(Vector) (Transformation|GetActorLocation) (Variables|Default|GetTarget)) (/ (Variables|Default|GetStartDistance2D) 2.0)))) false false))

(fn ConstructionScript)

(fn ChooseNewTargetAfterPush
  (params (PushedTeam :type ENUM_Teams%20Enum :default "NewEnumerator0"))
  (bind _localarrayplayer (LocalVariables|GetLocalArrayPlayer))
  (bind _outitem (Utilities|Array|Random _localarrayplayer))
  (bind _outactors (Actor|GetAllActorsOfClass "/Game/Valleyball/Blueprints/Pawn/BP_BaseValleyBallPawn.BP_BaseValleyBallPawn_C"))
  (for _array_element _outactors
    ;[1 1 1] Функционал, чтобы мяч прилетал гарантированно к игроку через n ударов
    (if (and (>= (Variables|Default|GetQualSelectedBot) (Variables|Default|GetMaxSelectBot)) (Utilities|Enum|Equal(Enum) PushedTeam "NewEnumerator1"))
      (if (Variables|/Game/Valleyball/Blueprints/Pawn/BP_BaseValleyBallPawn.BP_BaseValleyBallPawn_C|GetIsPlayer _array_element)
        (Utilities|Array|Add (LocalVariables|GetLocalArrayPlayer) _array_element))
      (elif (Utilities|Enum|NotEqual(Enum) PushedTeam (Variables|/Game/Valleyball/Blueprints/Pawn/BP_BaseValleyBallPawn.BP_BaseValleyBallPawn_C|GetTeam _array_element))
        (Utilities|Array|Add (LocalVariables|GetLocalArrayPlayer) _array_element))))
  (if (Variables|/Game/Valleyball/Blueprints/Pawn/BP_BaseValleyBallPawn.BP_BaseValleyBallPawn_C|GetIsPlayer _outitem)
    (Variables|Default|SetQualSelectedBot 0)
    (else
      (Variables|Default|SetQualSelectedBot (+ (Variables|Default|GetQualSelectedBot) 1))))
  (return (Transformation|GetActorLocation _outitem)))